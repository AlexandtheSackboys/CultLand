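; BP_Spawner is a spawner actor that repeatedly creates waves of actors around its own location.
; BeginPlay starts a looping timer that calls SpawnWave every few seconds for as long as it runs.
; Each wave spawns ObjectsPerWave actors at random horizontal offsets within a square centered on the spawner, at the spawner's height.
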(event EventBeginPlay
  (Utilities|Time|SetTimerbyFunctionName 0 "SpawnWave" 3.0 true))

(event Collision|EventActorBeginOverlap
  (params (OtherActor :type Actor%20Object%20Reference)))

(event EventTick
  (params (DeltaSeconds :type Float%20%28single-precision%29)))

(fn ConstructionScript)

(fn SpawnWave
  (for _index (range 0 (- (Variables|Default|GetObjectsPerWave) 1))
    (Game|SpawnActorfromClass "/Game/Callum_Content/BP_SpawnedObject.BP_SpawnedObject_C" (Math|Transform|MakeTransform (+ (Transformation|GetActorLocation) (Math|Vector|MakeVector (Math|Random|RandomFloatinRange -6e+02 6e+02) (Math|Random|RandomFloatinRange -6e+02 6e+02) 0.0)) "0, 0, 0" "1.000000,1.000000,1.000000") "Undefined" "MultiplyWithRoot" 0 0)))