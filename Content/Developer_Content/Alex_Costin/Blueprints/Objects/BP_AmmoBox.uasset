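; BP_AmmoBox is an ammo pickup that calls CollectAmmo whenever an actor overlaps it, without filtering which actor.
; On BeginPlay it caches the BP_ShooterWeaponBase returned by GetActorOfClass, then toggles its point light's visibility once through LightSwitch.
; The overlap passes that cached weapon's ammo reserve and magazine size to CollectAmmo, whose logic is not defined in this graph.
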(event EventBeginPlay
  (bind _returnvalue (Actor|GetActorOfClass "/Game/Variant_Shooter/Blueprints/Pickups/BP_ShooterWeaponBase.BP_ShooterWeaponBase_C"))
  (Variables|Default|Set_baseWeaponObject _returnvalue)
  (CallFunction|LightSwitch))

(event Collision|EventActorBeginOverlap
  (params (OtherActor :type Actor%20Object%20Reference))
  (bind __baseweaponobject (Variables|Default|Get_baseWeaponObject))
  (Class|AmmoCollectionPoint|CollectAmmo (Variables|/Game/Variant_Shooter/Blueprints/Pickups/BP_ShooterWeaponBase.BP_ShooterWeaponBase_C|GetAmmoReserve __baseweaponobject) (Variables|/Game/Variant_Shooter/Blueprints/Pickups/BP_ShooterWeaponBase.BP_ShooterWeaponBase_C|GetMag%20Size __baseweaponobject)))

(event EventTick
  (params (DeltaSeconds :type Float%20%28single-precision%29)))

(fn ConstructionScript)

(fn LightSwitch
  (Rendering|ToggleVisibility (Variables|Default|GetPointLight) false))