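; BP_FreezeExplosive is a projectile Blueprint that spawns a freeze explosion when it hits.
; On BeginPlay it zeroes the inherited projectile damage and allows damage to its owner.
; Its hit event spawns BP_FreezeExplosion at the projectile's transform regardless of collision, without calling any parent hit logic.
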(event EventBeginPlay
  (|CallParentFunction)
  (Variables|Default|Set_projectileDamage 0.0)
  (Variables|Default|Set_canDamageOwner true))

(event Collision|EventActorBeginOverlap
  (params (OtherActor :type Actor%20Object%20Reference))
  (|CallParentFunction OtherActor))

(event EventTick
  (params (DeltaSeconds :type Float%20%28single-precision%29))
  (|CallParentFunction DeltaSeconds) ; This node is disabled and will not be called.\nDrag off pins to build functionality.
)

(event EventOnProjectileHit
  (params (Hit :type Hit%20Result%20Structure%20%28by%20ref%29))
  (Game|SpawnActorfromClass "/Game/Developer_Content/Alex_Costin/Blueprints/Objects/BP_FreezeExplosion.BP_FreezeExplosion_C" (Transformation|GetActorTransform) "AlwaysSpawn" "MultiplyWithRoot" 0 0))

(fn ConstructionScript
  (|CallParentFunction))