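; BP_IceStaff is an ice staff weapon for the shooter, built as a child of a parent weapon Blueprint.
; On BeginPlay, the swap-weapon input or a touch switch, it sets a small clip with no reserve, enables projectile shooting and disables ammo collection.
; It contains only this configuration, with no firing logic of its own.
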(event Input|EnhancedActionEvents|EnhancedInputActionIA_SwapWeapon
  (params (ActionValue :type Boolean) (ElapsedSeconds :type Float%20%28double-precision%29) (TriggeredSeconds :type Float%20%28double-precision%29) (InputAction :type Input%20Action%20Object%20Reference :default "/Game/Variant_Shooter/Input/Actions/IA_SwapWeapon.IA_SwapWeapon"))
  (CallFunction|StartingAmmoSetup 5)
  (Variables|Default|SetIsShootingProjectile true)
  (Variables|Default|SetCanCollectAmmo false))

(event EventBeginPlay
  (|CallParentFunction)
  (CallFunction|StartingAmmoSetup 5)
  (Variables|Default|SetIsShootingProjectile true)
  (Variables|Default|SetCanCollectAmmo false))

(event Collision|EventActorBeginOverlap
  (params (OtherActor :type Actor%20Object%20Reference))
  (|CallParentFunction OtherActor) ; This node is disabled and will not be called.\nDrag off pins to build functionality.
)

(event EventTick
  (params (DeltaSeconds :type Float%20%28single-precision%29))
  (|CallParentFunction DeltaSeconds) ; This node is disabled and will not be called.\nDrag off pins to build functionality.
)

(event EventTouchSwitchWeapon
  (CallFunction|StartingAmmoSetup 5)
  (Variables|Default|SetIsShootingProjectile true)
  (Variables|Default|SetCanCollectAmmo false))

(fn ConstructionScript
  (|CallParentFunction))