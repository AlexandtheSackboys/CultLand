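; Shotgun weapon Blueprint for the shooter, a child weapon class that fires spread hit-scan shots instead of projectiles.
; BeginPlay selects the spread hit-scan class, runs parent setup, then applies hit-scan mode, range and damage from Launcher-named variables and enables ammo collection.
; The swap-weapon input and touch switch event reapply those same settings.
; RotateWeapon applies a given rotation to both first- and third-person weapon components.
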(event Input|EnhancedActionEvents|EnhancedInputActionIA_SwapWeapon
  (params (ActionValue :type Boolean) (ElapsedSeconds :type Float%20%28double-precision%29) (TriggeredSeconds :type Float%20%28double-precision%29) (InputAction :type Input%20Action%20Object%20Reference :default "/Game/Variant_Shooter/Input/Actions/IA_SwapWeapon.IA_SwapWeapon"))
  (Variables|Default|SetIsShootingProjectile false)
  (Variables|Default|SetRayCastRange (Variables|Default|Get_launcherRange))
  (Variables|Default|SetRayCastDamage (Variables|Default|Get_launcherDamage))
  (Variables|Default|SetCanCollectAmmo true))

(event EventBeginPlay
  (CallFunction|SetHitScanClass)
  (|CallParentFunction)
  (Variables|Default|SetIsShootingProjectile false)
  (Variables|Default|SetRayCastRange (Variables|Default|Get_launcherRange))
  (Variables|Default|SetRayCastDamage (Variables|Default|Get_launcherDamage))
  (Variables|Default|SetCanCollectAmmo true))

(event Collision|EventActorBeginOverlap
  (params (OtherActor :type Actor%20Object%20Reference))
  (|CallParentFunction OtherActor) ; This node is disabled and will not be called.\nDrag off pins to build functionality.
)

(event EventTick
  (params (DeltaSeconds :type Float%20%28single-precision%29))
  (|CallParentFunction DeltaSeconds) ; This node is disabled and will not be called.\nDrag off pins to build functionality.
)

(event EventTouchSwitchWeapon
  (Variables|Default|SetIsShootingProjectile false)
  (Variables|Default|SetRayCastRange (Variables|Default|Get_launcherRange))
  (Variables|Default|SetRayCastDamage (Variables|Default|Get_launcherDamage))
  (Variables|Default|SetCanCollectAmmo true))

(fn ConstructionScript
  (|CallParentFunction))

(fn RotateWeapon
  (params (StartRotation :type Rotator))
  (Transformation|SetWorldTransform (Variables|Default|GetFP_Weapon) (Math|Transform|MakeTransform "0, 0, 0" StartRotation "1.000000,1.000000,1.000000") false false)
  (Transformation|SetWorldTransform (Variables|Default|GetTP_Weapon) (Math|Transform|MakeTransform "0, 0, 0" StartRotation "1.000000,1.000000,1.000000") false false))

(fn SetHitScanClass
  (Variables|Default|SetHitScanBase (Variables|Default|GetBP_SpreadHitScan)))