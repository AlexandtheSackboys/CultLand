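; Pickup randomiser component that picks a weapon from WackWeaponList for the shooter.
; On BeginPlay it caches the list length as MaxWeaponIndex and prints it as text.
; WeaponPicker passes that value to Randomizer, whose body is not shown, then returns the list entry at RandomWeaponIndex.
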(event EventBeginPlay
  (bind _output_get (Variables|Default|SetMaxWeaponIndex (Utilities|Array|Length (Variables|Default|GetWackWeaponList))))
  (Development|PrintText (Utilities|Text|ToText(Integer) _output_get)))

(event EventTick
  (params (DeltaSeconds :type Float%20%28single-precision%29)))

(fn WeaponPicker
  (Class|WeaponPickupRandomizer|Randomizer (Variables|Default|GetMaxWeaponIndex))
  (return (Utilities|Array|Get(acopy) (Variables|Default|GetWackWeaponList) (Variables|Default|GetRandomWeaponIndex))))