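; BP_EnemySpawner is an enemy spawner that runs waves on a timer and shows the wave number on the HUD.
; BeginPlay seeds the current enemy count from the per-wave count and starts a looping timer at the spawn delay interval.
; Each tick of that timer runs WaveDelay, which calls SpawnWave, then writes WaveNumber into the shooter UI through the player's BP_WaveUI HUD.
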(event EventBeginPlay
  (Variables|Default|SetCurrentEnemyCount (Variables|Default|Get_enemiesPerWave))
  (Utilities|Time|SetTimerbyFunctionName 0 "WaveDelay" (Variables|Default|Get_spawnDelay) true))

(event Collision|EventActorBeginOverlap
  (params (OtherActor :type Actor%20Object%20Reference)))

(event EventTick
  (params (DeltaSeconds :type Float%20%28single-precision%29)))

(fn ConstructionScript)

(fn WaveDelay
  (Class|WaveSpawner|SpawnWave)
  (CallFunction|UpdateWaveUI))

(fn UpdateWaveUI
  (bind _asbp_wave_ui (Utilities|Casting|CastToBP_WaveUI (HUD|GetHUD (Game|GetPlayerController 0))))
  (Variables|/Game/Variant_Shooter/UI/UI_Shooter.UI_Shooter_C|SetWaveValueUI (Variables|/Game/Developer_Content/Alex_Costin/Blueprints/UI_Blueprints/BP_WaveUI.BP_WaveUI_C|GetShooterGameUI _asbp_wave_ui) (Utilities|Text|ToText(Integer) (Variables|Default|GetWaveNumber))))