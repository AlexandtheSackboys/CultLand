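; BP_ProjectileMaster is a projectile Blueprint, named as a master class, that damages what it hits and then destroys itself.
; On BeginPlay its collision sphere ignores the Instigator while moving.
; On hit it applies ProjectileDamage, disables collision and fires a radial force impulse.
; It then spawns an emitter aligned to the surface normal and plays the first-person template weapon-fire sound at the impact point.
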(event OnComponentHit(Sphere)
  (params (HitComponent :type Primitive%20Component%20Object%20Reference) (OtherActor :type Actor%20Object%20Reference) (OtherComp :type Primitive%20Component%20Object%20Reference) (NormalImpulse :type Vector :default "0, 0, 0") (Hit :type Hit%20Result%20Structure%20%28by%20ref%29))
  (bind (_bblockinghit _binitialoverlap _time _distance _location _impactpoint _normal) (Collision|BreakHitResult Hit))
  (Game|Damage|ApplyDamage OtherActor (Variables|Default|GetprojectileDamage) 0 self)
  (Collision|SetCollisionEnabled (Variables|Default|GetSphere) "NoCollision")
  (Class|RadialForceComponent|FireImpulse (Variables|Default|GetRadialForce))
  (Effects|SpawnEmitteratLocation 0 _location (Math|Rotator|MakeRotfromX _normal))
  (Audio|PlaySoundatLocation "/Game/Weapons/GrenadeLauncher/Audio/FirstPersonTemplateWeaponFire02.FirstPersonTemplateWeaponFire02" _location "0, 0, 0" 1.0 1.0 0.0 0 0 0 0)
  (Actor|DestroyActor))

(event EventBeginPlay
  (Collision|IgnoreActorwhenMoving (Variables|Default|GetSphere) (Game|GetInstigator) true))

(event Collision|EventActorBeginOverlap
  (params (OtherActor :type Actor%20Object%20Reference)))

(event EventTick
  (params (DeltaSeconds :type Float%20%28single-precision%29)))

(fn ConstructionScript)