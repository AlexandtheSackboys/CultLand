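; BP_Spawner is a prototype wave spawner for follow enemies that also reports the wave number to the HUD.
; A looping timer calls WaitSpawn, which runs SpawnWave and then updates the shooter UI through BP_WaveUI.
; SpawnWave spawns a batch at random horizontal offsets around itself only when CurrentObjectCount reaches zero, then resets the count and increments the wave.
; The count starts full and is never decremented within this Blueprint.
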(event EventBeginPlay
  (Variables|Default|SetCurrentObjectCount (Variables|Default|GetObjectsPerWave))
  (Utilities|Time|SetTimerbyFunctionName 0 "WaitSpawn" 5.0 true))

(event Collision|EventActorBeginOverlap
  (params (OtherActor :type Actor%20Object%20Reference)))

(event EventTick
  (params (DeltaSeconds :type Float%20%28single-precision%29)))

(fn ConstructionScript)

(fn SpawnWave
  (if (<= (Variables|Default|GetCurrentObjectCount) 0)
    (for _index (range 0 (- (Variables|Default|GetObjectsPerWave) 1))
      (Game|SpawnActorfromClass "/Game/Developer_Content/Alex_Costin/Blueprints/Characters/AI/BP_FollowEnemyPrototype.BP_FollowEnemyPrototype_C" (Math|Transform|MakeTransform (+ (Transformation|GetActorLocation) (Math|Vector|MakeVector (Math|Random|RandomFloatinRange -6e+02 6e+02) (Math|Random|RandomFloatinRange -6e+02 6e+02) 0.0)) "0, 0, 0" "1.000000,1.000000,1.000000") "Undefined" "MultiplyWithRoot" 0 0)
      (Variables|Default|SetCurrentObjectCount (Variables|Default|GetObjectsPerWave)))
    (bind _output_get (Variables|Default|Set_waveNumber (+ (Variables|Default|Get_waveNumber) 1)))
    (return _output_get)))

(fn UpdateWaveUI
  (params (waveValue :type Integer))
  (bind _asbp_wave_ui (Utilities|Casting|CastToBP_WaveUI (HUD|GetHUD (Game|GetPlayerController 0))))
  (Variables|/Game/Variant_Shooter/UI/UI_Shooter.UI_Shooter_C|SetWaveValueUI (Variables|/Game/Developer_Content/Alex_Costin/Blueprints/UI_Blueprints/BP_WaveUI.BP_WaveUI_C|GetShooterGameUI _asbp_wave_ui) (Utilities|Text|ToText(Integer) (Variables|Default|Get_waveNumber))))

(fn WaitSpawn
  (bind _wavenumber (CallFunction|SpawnWave))
  (CallFunction|UpdateWaveUI _wavenumber))