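; BP_Spawner is an actor that spawns a wave of BP_ShooterNPC characters around itself on BeginPlay.
; SpawnWave creates ObjectsPerWave NPCs at random X/Y offsets within a square centred on the spawner, at its height.
; An uncalled WaveManager function copies ObjectsPerWave into CurrentObjectCount and starts a looping SpawnWave timer only if that value is zero or less, so waves do not repeat.
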(event EventBeginPlay
  (CallFunction|SpawnWave))

(event Collision|EventActorBeginOverlap
  (params (OtherActor :type Actor%20Object%20Reference)))

(event EventTick
  (params (DeltaSeconds :type Float%20%28single-precision%29)))

(fn ConstructionScript)

(fn SpawnWave
  (for _index (range 0 (- (Variables|Default|GetObjectsPerWave) 1))
    (Game|SpawnActorfromClass "/Game/Variant_Shooter/Blueprints/AI/BP_ShooterNPC.BP_ShooterNPC_C" (Math|Transform|MakeTransform (+ (Transformation|GetActorLocation) (Math|Vector|MakeVector (Math|Random|RandomFloatinRange -6e+02 6e+02) (Math|Random|RandomFloatinRange -6e+02 6e+02) 0.0)) "0, 0, 0" "1.000000,1.000000,1.000000") "Undefined" "MultiplyWithRoot" 0 0)))

(fn WaveManager
  (bind _output_get (Variables|Default|SetCurrentObjectCount (Variables|Default|GetObjectsPerWave)))
  (if (<= _output_get 0)
    (Utilities|Time|SetTimerbyFunctionName 0 "SpawnWave" 3.0 true)))